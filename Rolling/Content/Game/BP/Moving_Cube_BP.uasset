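; Moving cube actor that oscillates its static mesh along the world Y or X axis once a movement event is triggered from outside.
; Each event caches the current location, offsets it through its own timeline without sweep, then calls the opposite event on finish.
; MoveRight and MoveLeft are one-time opening legs into the MoveLeft2/MoveRight2 loop, while MoveForward and MoveBackward alternate directly.
; SetTimer sets the actor's CustomTimeDilation to scale its speed.
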(event Custom|MoveForward
  (Variables|Default|SetLocation (Transformation|GetWorldLocation (Variables|Debug|GetStaticMeshComponent)))
  (bind _move (Timeline|타임라인_3 PlayFromStart)
    (:Update
      (Transformation|SetWorldLocation (Variables|Debug|GetStaticMeshComponent) (+ (Variables|Default|GetLocation) (Math|Vector|MakeVector _move 0.0 0.0)) false false))
    (:Finished
      (CallFunction|MoveBackward))))

(event Custom|MoveLeft
  (Variables|Default|SetLocation (Transformation|GetWorldLocation (Variables|Debug|GetStaticMeshComponent)))
  (bind _move (Timeline|타임라인_0 PlayFromStart)
    (:Update
      (Transformation|SetWorldLocation (Variables|Debug|GetStaticMeshComponent) (- (Variables|Default|GetLocation) (Math|Vector|MakeVector 0.0 _move 0.0)) false false))
    (:Finished
      (CallFunction|MoveRight2))))

(event Custom|MoveRight
  (Variables|Default|SetLocation (Transformation|GetWorldLocation (Variables|Debug|GetStaticMeshComponent)))
  (bind _move (Timeline|MoveY PlayFromStart)
    (:Update
      (Transformation|SetWorldLocation (Variables|Debug|GetStaticMeshComponent) (+ (Variables|Default|GetLocation) (Math|Vector|MakeVector 0.0 _move 0.0)) false false))
    (:Finished
      (CallFunction|MoveLeft2))))

(event Custom|MoveRight2
  (Variables|Default|SetLocation (Transformation|GetWorldLocation (Variables|Debug|GetStaticMeshComponent)))
  (bind _move (Timeline|타임라인_1 PlayFromStart)
    (:Update
      (Transformation|SetWorldLocation (Variables|Debug|GetStaticMeshComponent) (+ (Variables|Default|GetLocation) (Math|Vector|MakeVector 0.0 _move 0.0)) false false))
    (:Finished
      (CallFunction|MoveLeft2))))

(event Custom|MoveBackward
  (Variables|Default|SetLocation (Transformation|GetWorldLocation (Variables|Debug|GetStaticMeshComponent)))
  (bind _move (Timeline|타임라인_4 PlayFromStart)
    (:Update
      (Transformation|SetWorldLocation (Variables|Debug|GetStaticMeshComponent) (- (Variables|Default|GetLocation) (Math|Vector|MakeVector _move 0.0 0.0)) false false))
    (:Finished
      (CallFunction|MoveForward))))

(event Custom|MoveLeft2
  (Variables|Default|SetLocation (Transformation|GetWorldLocation (Variables|Debug|GetStaticMeshComponent)))
  (bind _move (Timeline|타임라인_2 PlayFromStart)
    (:Update
      (Transformation|SetWorldLocation (Variables|Debug|GetStaticMeshComponent) (- (Variables|Default|GetLocation) (Math|Vector|MakeVector 0.0 _move 0.0)) false false))
    (:Finished
      (CallFunction|MoveRight2))))

(event Custom|SetTimer
  (params (Timer :type Float%20%28single-precision%29))
  (Variables|Default|SetCustomTimeDilation Timer))

(event EventBeginPlay)

(event Collision|EventActorBeginOverlap
  (params (OtherActor :type Actor%20Object%20Reference)))

(event EventTick
  (params (DeltaSeconds :type Float%20%28single-precision%29)))

(fn ConstructionScript)