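; Movable cube actor whose color and rotation can be changed at runtime.
; The construction script creates a dynamic instance of the Color2_M material, which BeginPlay applies to the static mesh.
; ChangeColor sets that instance's BaseColor parameter, and the RandomRotate event gives the mesh a random world rotation without roll.
; Both are exposed for outside triggering, as nothing in this Blueprint calls them.
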(event Custom|Random%20Rotate
  (Transformation|SetWorldRotation (Variables|Debug|GetStaticMeshComponent) (Math|Random|RandomRotator false) false false))

(event EventBeginPlay
  (Rendering|Material|SetMaterial (Variables|Debug|GetStaticMeshComponent) 0 (Variables|Default|GetMaterial%20Instance)))

(event Collision|EventActorBeginOverlap
  (params (OtherActor :type Actor%20Object%20Reference)))

(event EventTick
  (params (DeltaSeconds :type Float%20%28single-precision%29)))

(fn ConstructionScript
  (bind _returnvalue (Rendering|Material|CreateDynamicMaterialInstance "/Game/Game/Material/Color2_M.Color2_M" :!class /Script/Engine.KismetMaterialLibrary))
  (Variables|Default|SetMaterial%20Instance _returnvalue))

(fn ChangeColor
  (params (Color :type Linear%20Color%20Structure))
  (Rendering|Material|SetVectorParameterValue (Variables|Default|GetMaterial%20Instance) "BaseColor" Color :!class /Script/Engine.MaterialInstanceDynamic))