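; Movable_Cubes_BP is a spawner actor that lays out a flat checkerboard grid of two movable cube Blueprints.
; The Construction Script loops over rows and adds evenly spaced Child Actor Components in pairs, alternating Movable_Cube_BP and Movable_Cube2_BP along each row.
; A FlipFlop swaps the pair order on every other row to produce the checker pattern.
; The Event Graph holds only disabled placeholder events, so this Blueprint adds no runtime logic.
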(event EventBeginPlay)

(event Collision|EventActorBeginOverlap
  (params (OtherActor :type Actor%20Object%20Reference)))

(event EventTick
  (params (DeltaSeconds :type Float%20%28single-precision%29)))

(fn ConstructionScript
  (for _index (range 0 14)
    (Utilities|FlowControl|FlipFlop
      (:A
        (for _index_2 (range 0 6)
          (bind _returnvalue (AddComponent|AddChildActorComponent false (Math|Transform|MakeTransform (Math|Vector|MakeVector (* _index_2 3.8e+02) (* _index 1.9e+02) 75.0))))
          (ChildActorComponent|SetChildActorClass _returnvalue "/Game/Game/BP/Movable_Cube_BP.Movable_Cube_BP_C")
          (bind _returnvalue_2 (AddComponent|AddChildActorComponent false (Math|Transform|MakeTransform (Math|Vector|MakeVector (+ (* _index_2 3.8e+02) 1.9e+02) (* _index 1.9e+02) 75.0))))
          (ChildActorComponent|SetChildActorClass _returnvalue_2 "/Game/Game/BP/Movable_Cube2_BP.Movable_Cube2_BP_C")))
      (:B
        (for _index_3 (range 0 6)
          (bind _returnvalue_3 (AddComponent|AddChildActorComponent false (Math|Transform|MakeTransform (Math|Vector|MakeVector (* _index_3 3.8e+02) (* _index 1.9e+02) 75.0))))
          (ChildActorComponent|SetChildActorClass _returnvalue_3 "/Game/Game/BP/Movable_Cube2_BP.Movable_Cube2_BP_C")
          (bind _returnvalue_4 (AddComponent|AddChildActorComponent false (Math|Transform|MakeTransform (Math|Vector|MakeVector (+ (* _index_3 3.8e+02) 1.9e+02) (* _index 1.9e+02) 75.0))))
          (ChildActorComponent|SetChildActorClass _returnvalue_4 "/Game/Game/BP/Movable_Cube_BP.Movable_Cube_BP_C"))))))