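; Black hole actor whose material pulses in edge sharpness on a repeating cycle.
; The construction script creates a dynamic instance of Blackhole_M, which BeginPlay applies to the static mesh before starting a looping Impulse timer.
; Each Impulse plays a timeline that drives the Edge Sharpness parameter, then adds a child actor component when finished.
; A ChangeColor helper sets BaseColor but is not called here.
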(event OnComponentHit(StaticMeshComponent)
  (params (HitComponent :type Primitive%20Component%20Object%20Reference) (OtherActor :type Actor%20Object%20Reference) (OtherComp :type Primitive%20Component%20Object%20Reference) (NormalImpulse :type Vector :default "0, 0, 0") (Hit :type Hit%20Result%20Structure%20%28by%20ref%29)))

(event Custom|Impulse
  (bind _sharpness (Timeline|타임라인_0 PlayFromStart)
    (:Update
      (CallFunction|ChangeSharpness _sharpness))
    (:Finished
      (AddComponent|AddChildActorComponent false))))

(event EventBeginPlay
  (Rendering|Material|SetMaterial (Variables|Debug|GetStaticMeshComponent) 0 (Variables|Default|GetMaterial%20Instance))
  (CallFunction|Impulse)
  (Utilities|Time|SetTimerbyFunctionName 0 "Impulse" 3.5 true))

(event Collision|EventActorBeginOverlap
  (params (OtherActor :type Actor%20Object%20Reference)))

(event EventTick
  (params (DeltaSeconds :type Float%20%28single-precision%29)))

(fn ConstructionScript
  (bind _returnvalue (Rendering|Material|CreateDynamicMaterialInstance "/Game/Game/Material/Blackhole_M.Blackhole_M" :!class /Script/Engine.KismetMaterialLibrary))
  (Variables|Default|SetMaterial%20Instance _returnvalue))

(fn ChangeColor
  (params (Color :type Linear%20Color%20Structure))
  (Rendering|Material|SetVectorParameterValue (Variables|Default|GetMaterial%20Instance) "BaseColor" Color :!class /Script/Engine.MaterialInstanceDynamic))

(fn ChangeSharpness
  (params (Edge :type Float%20%28single-precision%29))
  (Rendering|Material|SetScalarParameterValue (Variables|Default|GetMaterial%20Instance) "Edge Sharpness" Edge :!class /Script/Engine.MaterialInstanceDynamic))